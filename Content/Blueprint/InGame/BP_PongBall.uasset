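; BP_PongBall is the physics-driven Pong ball, launched with a fixed force on BeginPlay.
; Each hit plays a paddle or wall sound based on the hit actor's class.
; Left and right walls, matched by display name, add to the opposing score in GM_Pong, update that pawn's score UI and trigger brief slow motion.
; After a short delay, each hit also adds an impulse along the velocity, speeding up the ball.
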(event OnComponentHit(SphereCollision)
  (params (HitComponent :type Primitive%20Component%20Object%20Reference) (OtherActor :type Actor%20Object%20Reference) (OtherComp :type Primitive%20Component%20Object%20Reference) (NormalImpulse :type Vector :default "0, 0, 0") (Hit :type Hit%20Result%20Structure%20%28by%20ref%29))
  (bind (_bblockinghit _binitialoverlap _time _distance _location _impactpoint _normal _impactnormal _physmat _hitactor) (Collision|BreakHitResult Hit))
  (bind _returnvalue (Utilities|GetDisplayName OtherActor))
  (bind _gamemoderef (Variables|Default|GetgameModeRef))
  (bind _spherecollision (Variables|Default|GetSphereCollision))
  (Development|PrintString _returnvalue)
  (Utilities|FlowControl|Sequence
    (:then_0
      ;[1 1 1] Paly sounds
      (Utilities|Casting|CastToPongPawn _hitactor
        (:then
          (Audio|PlaySoundatLocation "/Game/Audio/SFX/Cue_Hit.Cue_Hit" _impactpoint "0, 0, 0" 1.0 1.0 0.0 0 0 0 0))
        (:CastFailed
          (Audio|PlaySoundatLocation "/Game/Audio/SFX/Cue_WallHit.Cue_WallHit" _impactpoint "0, 0, 0" 1.0 1.0 0.0 0 0 0 0))))
    (:then_1
      ;[1 1 1] add score
      (switch string _returnvalue
        (:WallLeft
          (bind _result (Math|Integer|IncrementInt (Variables|/Game/Blueprint/InGame/GM_Pong.GM_Pong_C|GetPlayer2Score _gamemoderef))
            (:%20%20
              (bind _aspong_pawn (Utilities|Casting|CastToPongPawn (Pawn|GetControlledPawn (Game|GetPlayerController 1))))
              (Default|OnUpdateScore (Variables|/Game/Blueprint/InGame/PongPawn.PongPawn_C|GetPlayerScoreUI _aspong_pawn) _result))))
        (:WallRight
          (bind _result_2 (Math|Integer|IncrementInt (Variables|/Game/Blueprint/InGame/GM_Pong.GM_Pong_C|GetPlayer1Score _gamemoderef))
            (:%20%20
              (bind _aspong_pawn_2 (Utilities|Casting|CastToPongPawn (Pawn|GetControlledPawn (Game|GetPlayerController 0))))
              (Default|OnUpdateScore (Variables|/Game/Blueprint/InGame/PongPawn.PongPawn_C|GetPlayerScoreUI _aspong_pawn_2) _result_2)))))
      (Utilities|Time|SetGlobalTimeDilation 0.2)
      (Utilities|FlowControl|Delay 0.1)
      (Utilities|Time|SetGlobalTimeDilation 1.0))
    (:then_2
      (Utilities|FlowControl|Delay 0.1)
      (if (Physics|IsSimulatingPhysics _spherecollision "None")
        (Physics|AddImpulse _spherecollision (* (Math|Vector|Normalize (Transformation|GetVelocity)) "200.000000,200.000000,200.000000") "None" true)))))

(event EventBeginPlay
  (bind _spherecollision (Variables|Default|GetSphereCollision))
  (bind _asgm_pong (Utilities|Casting|CastToGM_Pong (Game|GetGameMode)))
  (Variables|Default|SetgameModeRef _asgm_pong)
  (Physics|SetSimulatePhysics _spherecollision true)
  (Physics|AddForce _spherecollision "100000.000000,90000.000000, 0" "None" true)
  (Development|PrintString "Hello"))

(fn ConstructionScript)