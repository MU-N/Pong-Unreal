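; PongPawn is the player-controlled paddle pawn for a Pong game.
; The PongVerticalMove input axis sets a move direction, and Tick applies it as a swept local X offset scaled by move speed and delta time.
; BeginPlay casts and stores a reference to the GM_Pong game mode, which the pawn's graph does not otherwise use.
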(event EventBeginPlay
  (bind _asgm_pong (Utilities|Casting|CastToGM_Pong (Game|GetGameMode)))
  (Variables|Default|SetGameModeRef _asgm_pong))

(event Collision|EventActorBeginOverlap
  (params (OtherActor :type Actor%20Object%20Reference)))

(event EventTick
  (params (DeltaSeconds :type Float%20%28single-precision%29))
  (Transformation|AddActorLocalOffset (Math|Vector|MakeVector (* (* DeltaSeconds (Variables|Default|GetMoveDirection)) (Variables|Default|GetMoveSpeed)) 0.0 0.0) true false))

(event Input|ActionEvents|InputActionPongPuase
  (params (Key :type Key%20Structure :default "None")))

(event Input|AxisEvents|InputAxisPongVerticalMove
  (params (AxisValue :type Float%20%28single-precision%29))
  (Variables|Default|SetMoveDirection AxisValue))

(fn ConstructionScript)