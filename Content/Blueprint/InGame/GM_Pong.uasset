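; Game mode for local multiplayer Pong that sets up one player per PlayerStart when play begins.
; It creates a local player for each start found in the level, then moves each controller's pawn to the matching start location.
; Each PongPawn's cube gets a dynamic material instance tinted from the PlayerColors array by player index.
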(event EventBeginPlay
  ;[1 1 1] Players Controllers
  (bind _outactors (Actor|GetAllActorsOfClass "/Script/Engine.PlayerStart"))
  (if (!= (Utilities|Array|Length _outactors) 0)
    (for (_ _array_index) _outactors
      (Class|GameplayStatics|CreatePlayer _array_index))
    ;[1 1 1] set difrent location for each player
    (for (_array_element _array_index_2) _outactors
      (Transformation|SetActorLocation (Pawn|GetControlledPawn (Game|GetPlayerController _array_index_2)) (Transformation|GetActorLocation _array_element) false false)
      ;[1 1 1] Change matrilas for palayers
      (bind _aspong_pawn (Utilities|Casting|CastToPongPawn (Pawn|GetControlledPawn (Game|GetPlayerController _array_index_2))))
      (bind _returnvalue (Rendering|Material|CreateDynamicMaterialInstance (Variables|/Game/Blueprint/InGame/PongPawn.PongPawn_C|GetCube _aspong_pawn) 0 (Rendering|Material|GetMaterial (Variables|/Game/Blueprint/InGame/PongPawn.PongPawn_C|GetCube _aspong_pawn) 0) "None" :!class /Script/Engine.PrimitiveComponent))
      (Rendering|Material|SetVectorParameterValue _returnvalue "Color" (Utilities|Array|Get(acopy) (Variables|Default|GetPlayerColors) _array_index_2) :!class /Script/Engine.MaterialInstanceDynamic)
      (Rendering|Material|SetMaterial (Variables|/Game/Blueprint/InGame/PongPawn.PongPawn_C|GetCube _aspong_pawn) 0 _returnvalue))))

(event EventTick
  (params (DeltaSeconds :type Float%20%28single-precision%29)))

(fn ConstructionScript)